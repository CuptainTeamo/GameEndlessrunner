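; Player character for a side-scrolling auto-runner with flipbook animation, which moves along +X every tick.
; Jump and crouch input drive jump and slide flipbooks, with crouch also offsetting and rotating the sprite and jump returning to run on a fixed delay rather than on landing.
; Damage lowers Health and refreshes the HUD created on BeginPlay; exactly zero Health stops movement and shows idle.
; The construction script derives HeartContainers from Health.
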(event `InputAction|Crouch`
  (params (Key :type "Key Structure"))
  (bind _sprite (`self.Sprite`))
  (bind _sprite_2 (`self.Sprite`))
  ;[1 1 1] Crouch and animation
  (:`Pressed`
    (`self.Crouch`)
    (`SceneComponent.K2_SetRelativeLocation` (`self.Sprite`) (0.0 0.0 -5.0) false false)
    (`SceneComponent.K2_SetRelativeRotation` _sprite_2 (struct :`Yaw` 180.0) false false)
    (`PaperFlipbookComponent.SetFlipbook` _sprite_2 "/Game/Assets/Characters/FB_Slide.FB_Slide"))
  (:`Released`
    (`self.UnCrouch`)
    (`SceneComponent.K2_SetRelativeLocation` (`self.Sprite`) (0.0 0.0 0.0) false false)
    (`SceneComponent.K2_SetRelativeRotation` :`self` _sprite)
    (`PaperFlipbookComponent.SetFlipbook` _sprite "/Game/Assets/Characters/FB_Run.FB_Run")))

(event `InputAction|Jump`
  (params (Key :type "Key Structure"))
  ;[1 1 1] Jump and set animation
  (:`Pressed`
    (if (`self.f_IsNotJumping`)
      (`self.Jump`)
      (`PaperFlipbookComponent.SetFlipbook` (`self.Sprite`) "/Game/Assets/Characters/FB_Jump.FB_Jump")
      (`KismetSystemLibrary.Delay` 0.6)
      (`PaperFlipbookComponent.SetFlipbook` (`self.Sprite`) "/Game/Assets/Characters/FB_Run.FB_Run"))))

(event `self.ReceiveBeginPlay`
  ;[1 1 1] Add Heart Widget
  (bind _returnvalue (`|CreateWidget` "/Game/Blueprints/UI/WB_PlayerHUD.WB_PlayerHUD_C"))
  (bind _output_get (set `self.PlayerHUD` _returnvalue))
  (`UserWidget.AddToViewport` _output_get 0))

(event `self.ReceiveTick`
  (params (DeltaSeconds :type "Float (single-precision)"))
  ;[1 1 1] Add Right Movement to player
  (`self.AddMovementInput` (0.2 0.0 0.0) (`self.Speed`))
  (if (== (`self.Health`) 0.0)
    (set `self.Speed` 0.0)))

(event `self.ReceiveAnyDamage`
  (params (Damage :type "Float (single-precision)") (DamageType :type "DamageType Object Reference") (InstigatedBy :type "Controller Object Reference") (DamageCauser :type "Actor Object Reference"))
  ;[1 1 1] Player take damage
  (set `self.Health` (- (`self.Health`) Damage))
  (`/Game/Blueprints/UI/WB_PlayerHUD.UpdateHealth` (`self.PlayerHUD`))
  (if (== (`self.Health`) 0.0)
    (`PaperFlipbookComponent.SetFlipbook` (`self.Sprite`) "/Game/Assets/Characters/FB_Idle.FB_Idle")))

(fn `f_IsNotJumping`
  (returns (ReturnValue :type Boolean))
  (return (not (`NavMovementComponent.IsFalling` (`self.CharacterMovement`)))))

(fn `UserConstructionScript`
  (set `self.HeartContainers` (`KismetMathLibrary.FTrunc` (`self.Health`))))