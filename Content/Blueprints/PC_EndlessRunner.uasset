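; Player controller for an endless runner that owns the main HUD and shows a death message.
; On BeginPlay it creates the WB_Main widget, stores it and adds it to the viewport.
; Every Tick it casts the player character to BP_Player and calls the widget's DisplayDeathMessage while Health equals zero, polling rather than reacting to an event.
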(event `self.ReceiveBeginPlay`
  (bind _returnvalue (`|CreateWidget` "/Game/Blueprints/UI/WB_Main.WB_Main_C"))
  (bind _output_get (set `self.WB_Main` _returnvalue))
  (`UserWidget.AddToViewport` _output_get 0))

(event `self.ReceiveTick`
  (params (DeltaSeconds :type "Float (single-precision)"))
  (bind _asbp_player (cast `/Game/Blueprints/BP_Player` (`GameplayStatics.GetPlayerCharacter` 0)))
  (if (== (`/Game/Blueprints/BP_Player.Health` _asbp_player) 0.0)
    (`/Game/Blueprints/UI/WB_Main.DisplayDeathMessage` (`self.WB_Main`))))

(fn `UserConstructionScript`)